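; Shooting range target for a VR game that scores shots and aim samples and can rotate its holder.
; GetHitData measures a hit in the Y/Z plane against the target midpoint, giving distance, angle and relative location.
; RegisterHit and RegisterAim send that data to ShootingRangeVRGameMode and return whether it falls within TargetRadius.
; RotateTarget moves the holder cylinder between two yaw angles, and HitTarget counts inside and outside hits.
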(event `self.ReceiveActorBeginOverlap`
  (params (OtherActor :type "Actor Object Reference")))

(event `RotateTarget`
  (params (IsTurned :type Boolean))
  (if IsTurned
    (set `self.RotationAmount` 180.0)
    (else
      (set `self.RotationAmount` 90.0)))
  (`KismetSystemLibrary.MoveComponentTo` (`self.TargetHolder_Cylinder`) (0.0 0.0 0.0) (`KismetMathLibrary.MakeRotator` 0.0 0.0 (`self.RotationAmount`))))

(fn `GetHitData`
  (params (HitLocation :type "Vector Structure"))
  (returns (HitDistance :type "Float (double-precision)") (HitAngle :type "Float (double-precision)") (RelativeHitLocation :type "Vector Structure"))
  (bind (_midpoint_x _midpoint_y _midpoint_z) (`KismetMathLibrary.BreakVector` (`self.MidPoint`)))
  (bind (_returnvalue_x _returnvalue_y _returnvalue_z) (`KismetMathLibrary.BreakVector` (`SceneComponent.K2_GetComponentLocation` (`self.DefaultSceneRoot`))))
  (bind _returnvalue (+ _midpoint_z _returnvalue_z))
  (bind _returnvalue_2 (+ _midpoint_y _returnvalue_y))
  (return (`KismetMathLibrary.Distance2D` (`KismetMathLibrary.MakeVector2D` HitLocation_Y HitLocation_Z) (`KismetMathLibrary.MakeVector2D` _returnvalue_2 _returnvalue)) (`KismetMathLibrary.Atan2` (- _midpoint_z HitLocation_Z) (- _midpoint_y HitLocation_Y)) (`KismetMathLibrary.MakeVector` 0.0 (- HitLocation_Y _returnvalue_2) (- HitLocation_Z _returnvalue))))

(fn `HitTarget`
  (params (Inside :type Boolean))
  (if Inside
    (`/Engine/EditorBlueprintResources/StandardMacros.IncrementInt` (`self.InsideCircleHits`))
    (else
      (`/Engine/EditorBlueprintResources/StandardMacros.IncrementInt` (`self.OutsideCircleHits`)))))

(fn `RegisterAim`
  (params (HitLocation :type "Vector Structure"))
  (returns (InsideCircle :type Boolean))
  (bind (_hitdistance _hitangle _relativehitlocation) (`self.GetHitData` HitLocation))
  (bind _returnvalue (`GameplayStatics.GetActorOfClass` "/Game/GameModes/ShootingRangeVRGameMode.ShootingRangeVRGameMode_C"))
  (`/Game/GameModes/ShootingRangeVRGameMode.AddAimResult` _returnvalue _relativehitlocation)
  (return (<= _hitdistance (`self.TargetRadius`))))

(fn `RegisterHit`
  (params (HitLocation :type "Vector Structure") (Round :type Integer))
  (returns (InsideCircle :type Boolean))
  (bind (_hitdistance _hitangle _relativehitlocation) (`self.GetHitData` HitLocation))
  (bind _returnvalue (`GameplayStatics.GetActorOfClass` "/Game/GameModes/ShootingRangeVRGameMode.ShootingRangeVRGameMode_C"))
  (`/Game/GameModes/ShootingRangeVRGameMode.AddResult` _returnvalue _hitdistance _hitangle Round _relativehitlocation)
  (return (<= _hitdistance (`self.TargetRadius`))))

(fn `TurnTarget`)

(fn `UserConstructionScript`)